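; BP_PL_WallCupboard1_Ice is a placeable wall cupboard whose inventory stops items perishing while it contains item template 18040, presumably ice.
; Inventory add, remove and stat-change signals re-check for that item and set PerishModifier to zero, or back to normal without it.
; On non-servers, BeginPlay creates a client inventory monitor and runs the same check when the inventory arrives.
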(event `self.ReceiveBeginPlay`
  (bind _placeableinventory (`self.PlaceableInventory`))
  (`parent.ReceiveBeginPlay`)
  (if (not (`KismetSystemLibrary.IsServer`))
    (bind _returnvalue (`|GenericCreateObject` "/Script/ConanSandbox.ItemInventoryClientMonitor" self))
    (bind _output_get (set `self.PlaceableInventoryMonitor` _returnvalue))
    (`ItemInventoryClientMonitor.SetInventory` _output_get _placeableinventory)
    (add `ItemInventory.SignalInventoryRecivedOnClient` _placeableinventory (delegate `UpdatePerishModifier`))))

(event `self.PlaceableInventory.SignalItemAdded`
  (params (index :type Integer) (item :type "GameItem Object Reference") (srcInventory :type "ItemInventory Object Reference") (srcIndex :type Integer))
  (if (`ItemInventory.HasItemByTemplateID` (`self.PlaceableInventory`) 18040 1) :!label _label
    (set `ItemInventory.PerishModifier` 0.0 (`self.PlaceableInventory`))
    (else
      (set `ItemInventory.PerishModifier` 1.0 (`self.PlaceableInventory`)))))

(event `UpdatePerishModifier`
  (goto _label))

(event `self.PlaceableInventory.SignalItemRemoved`
  (params (index :type Integer) (item :type "GameItem Object Reference") (dstInventory :type "ItemInventory Object Reference") (dstIndex :type Integer))
  (goto _label))

(event `self.PlaceableInventory.SignalItemFloatStatChanged`
  (params (item :type "GameItem Object Reference") (statID :type "EItemFloatStatID Enum" :default "WeaponStaminaHeavyChargedRegenModifier") (statValue :type "Float (single-precision)") (deltaValue :type "Float (single-precision)"))
  (goto _label))

(event `self.PlaceableInventory.SignalItemIntStatChanged`
  (params (item :type "GameItem Object Reference") (statID :type "EItemIntStatID Enum" :default "MaxStackSize") (statValue :type Integer) (deltaValue :type Integer))
  (goto _label))

(fn `UserConstructionScript`
  (`parent.UserConstructionScript`))